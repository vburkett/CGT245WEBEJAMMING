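; Spoon is a goal actor that drops from high above to a fixed spot when play begins, then ends the game with a win screen when the player touches it.
; A Timeline lerps its location between two hardcoded points and sets its scale once the descent finishes.
; Overlap with BP_ThirdPersonCharacter shows the Winscreen widget, switches to UI-only input with a visible cursor, and stops the character's movement.
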(event `self.ReceiveBeginPlay`
  (bind (_direction _newtrack_0) (`Timeline|Timeline` :!via `PlayFromStart`)
    (:`Update`
      (`self.K2_SetActorLocation` (`KismetMathLibrary.VLerp` (-460.0 -130.0 4190.0) (-460.0 -130.0 190.0) _newtrack_0)))
    (:`Finished`
      (`self.SetActorScale3D` (0.25 0.25 0.25)))))

(event `self.ReceiveActorBeginOverlap`
  (params (OtherActor :type "Actor Object Reference"))
  (bind _returnvalue (`GameplayStatics.GetPlayerController` 0))
  (bind _asbp_third_person_character (cast `/Game/ThirdPerson/Blueprints/BP_ThirdPersonCharacter` OtherActor))
  (bind _returnvalue_2 (`|CreateWidget` "/Game/Blueprints/winscreen.winscreen_C"))
  (`UserWidget.AddToViewport` _returnvalue_2 0)
  (`WidgetBlueprintLibrary.SetInputMode_UIOnlyEx` _returnvalue _returnvalue_2)
  (set `PlayerController.bShowMouseCursor` true _returnvalue)
  (`MovementComponent.StopMovementImmediately` (`Character.CharacterMovement` _asbp_third_person_character)))

(fn `UserConstructionScript`)